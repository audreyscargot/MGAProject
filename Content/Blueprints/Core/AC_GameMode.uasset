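; AC_GameMode is a game mode component, judging by its name, that runs level sequences with quick-time event (QTE) pauses.
; It tracks the current sequence actor, and PlayLevelSequence destroys the previous one before playing another.
; Registering a montage shows the QTE widget, switches to limited input mapping and pauses the sequence.
; PlayAnimMontage resumes it, jumping the player character's montage to its "Next" section.
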(fn `DestroyPreviousLevelSequence`
  (bind _currentlevelsequenceactor (`self.CurrentLevelSequenceActor`)
    (:`then`
      (`Actor.K2_DestroyActor` _currentlevelsequenceactor))
    (:`else`
      _))
  (return))

(fn `PlayAnimMontage`
  (`AnimInstance.Montage_JumpToSection` (`SkeletalMeshComponent.GetAnimInstance` (`/Game/Blueprints/Characters/Components/AC_CharacterComponent.Body` (`Actor.GetComponentByClass` (`GameplayStatics.GetPlayerCharacter` 0) "/Game/Blueprints/Characters/Components/AC_CharacterComponent.AC_CharacterComponent_C"))) "Next" (`self.Current Montage`))
  (`MovieSceneSequencePlayer.Play` (`LevelSequenceActor.SequencePlayer` (`self.CurrentLevelSequenceActor`)))
  (return))

(fn `PlayLevelSequence`
  (params (LevelSequence :type "LevelSequence Object Reference") (`Settings Pause At End` :type Boolean :default true))
  (`|ExecutionSequence`
    (:`then_0`
      (`self.DestroyPreviousLevelSequence`))
    (:`then_1`
      (bind _outactor (`LevelSequencePlayer.CreateLevelSequencePlayer` LevelSequence (make `MovieSceneSequencePlaybackSettings` false (struct) (struct :`bAllowRounding` true) 1.0 0.0 false false false false false false "None" `Settings Pause At End`)))
      (`MovieSceneSequencePlayer.Play` (`LevelSequenceActor.SequencePlayer` _outactor))
      (set `self.CurrentLevelSequenceActor` _outactor))))

(fn `RegisterCurrentMontage`
  (params (CurrentMontage :type "AnimMontage Object Reference"))
  (set `self.Current Montage` CurrentMontage)
  (`self.StartQTE`)
  (`MovieSceneSequencePlayer.Pause` (`LevelSequenceActor.SequencePlayer` (`self.CurrentLevelSequenceActor`))))

(fn `StartLevelSequence`
  (params (LevelSequence :type "LevelSequence Object Reference"))
  (bind _outactor (`LevelSequencePlayer.CreateLevelSequencePlayer` LevelSequence (make `MovieSceneSequencePlaybackSettings` true)))
  (set `self.CurrentLevelSequenceActor` _outactor))

(fn `StartQTE`
  (bind _returnvalue (`|CreateWidget` "/Game/Blueprints/Widgets/WBP_QTE.WBP_QTE_C" null null null))
  (`UserWidget.AddToViewport` _returnvalue 0)
  (bind _asbp_third_person_player_controller (cast `/Game/Blueprints/Core/BP_ThirdPersonPlayerController` (`GameplayStatics.GetPlayerController` 0)))
  (`/Game/Blueprints/Core/BP_ThirdPersonPlayerController.UpdateInputMapping` _asbp_third_person_player_controller "/Game/Input/IMC_Limited.IMC_Limited" "/Game/Input/IMC_Default.IMC_Default"))
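; Character component that clamps camera view pitch and lets the player interact with objects in view.
; InitializeCamera stores the camera and enables tick, which runs a debug-drawn forward line trace to track the targeted BP_InteractableBase, clearing it on a miss.
; IA_Interact calls Interact on that target with the player character, while IA_LimitedInteract broadcasts LimitedInteractHasBeenPressed.
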(event `self.ReceiveBeginPlay`
  (bind _returnvalue (`GameplayStatics.GetPlayerCameraManager` 0))
  (set `PlayerCameraManager.ViewPitchMin` (`self.View Pitch Min`) _returnvalue)
  (set `PlayerCameraManager.ViewPitchMax` (`self.View Pitch Max`) _returnvalue))

(event `InitializeCamera`
  (params (CameraActor :type "CameraComponent Object Reference"))
  (bind _output_get (set `self.CameraActor` CameraActor))
  (`/Engine/EditorBlueprintResources/StandardMacros.IsValid` _output_get
    (:`Is Valid`
      (`self.SetComponentTickEnabled` true))))

(event `self.ReceiveTick`
  (params (DeltaSeconds :type "Float (single-precision)"))
  (bind _cameraactor (`self.CameraActor`))
  (bind _returnvalue (`SceneComponent.K2_GetComponentLocation` _cameraactor))
  (bind _outhit (`KismetSystemLibrary.LineTraceSingle` :`Start` _returnvalue :`End` (+ _returnvalue (* (`SceneComponent.GetForwardVector` _cameraactor) (`self.TraceLength`))) :`TraceChannel` "TraceTypeQuery3" :`DrawDebugType` "ForOneFrame"))
  (bind (_bblockinghit _binitialoverlap _time _distance _location _impactpoint _normal _impactnormal _physmat _hitactor) (`GameplayStatics.BreakHitResult` _outhit))
  (if _bblockinghit
    (if (!= _hitactor (`self.InteractTarget`))
      (bind _asbp_interactable_base (cast `/Game/Blueprints/Objects/Interactable/BP_InteractableBase` _hitactor))
      (set `self.InteractTarget` _asbp_interactable_base))
    (else
      (set `self.InteractTarget` null))))

(event `EnhancedInput|/Game/Input/Actions/IA_Interact`
  (params (ActionValue :type Boolean) (ElapsedSeconds :type "Float (double-precision)") (TriggeredSeconds :type "Float (double-precision)") (InputAction :type "InputAction Object Reference" :default "/Game/Input/Actions/IA_Interact.IA_Interact"))
  (:`Started`
    (bind _interacttarget (`self.InteractTarget`)
      (:`then`
        (`/Game/Blueprints/Objects/Interactable/BP_InteractableBase.Interact` _interacttarget (`GameplayStatics.GetPlayerCharacter` 0)))
      (:`else`))))

(event `EnhancedInput|/Game/Input/Actions/IA_LimitedInteract`
  (params (ActionValue :type Boolean) (ElapsedSeconds :type "Float (double-precision)") (TriggeredSeconds :type "Float (double-precision)") (InputAction :type "InputAction Object Reference" :default "/Game/Input/Actions/IA_LimitedInteract.IA_LimitedInteract"))
  (:`Started`
    (`self.LimitedInteractHasBeenPressed` self)))
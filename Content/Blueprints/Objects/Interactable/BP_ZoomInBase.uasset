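; Base interactable that zooms the view onto a readable document and shows its title and text in a WBP_TextTranslation widget.
; Interact swaps input to IMC_Limited and uses a timed camera fade before moving the view target to this actor and opening the widget.
; The limited-interact event is bound for exit, and CloseInteract works only after the widget signals CanQuit, then fades back to the player and restores default input.
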(event `CameraEffect`
  (params (isOpening :type Boolean :default true))
  (bind _returnvalue (`GameplayStatics.GetPlayerCameraManager` 0))
  ; Open/Close Document Effect
  (`PlayerCameraManager.StartCameraFade` :`self` _returnvalue :`ToAlpha` 1.0 :`Duration` 0.5 :`bHoldWhenFinished` true)
  (`KismetSystemLibrary.Delay` 0.5)
  (`PlayerCameraManager.StartCameraFade` :`self` _returnvalue :`FromAlpha` 1.0 :`Duration` 1.0 :`bHoldWhenFinished` true)
  (if isOpening
    (`self.OpenDoc`)
    (else
      (`self.CloseDoc`))))

(event `OpenDoc`
  ; Open/Close Document Effect
  (bind _returnvalue (`|CreateWidget` "/Game/Blueprints/Widgets/WBP_TextTranslation.WBP_TextTranslation_C" null (`self.Document Text`) (`self.Title Text`)))
  (bind _output_get (set `self.WidgetTextRef` _returnvalue))
  (add `/Game/Blueprints/Widgets/WBP_TextTranslation.CanQuitUpdate` _output_get (delegate `CanQuitUpdate`))
  (`UserWidget.AddToViewport` _output_get 0)
  (`PlayerController.SetViewTargetWithBlend` (`GameplayStatics.GetPlayerController` 0) self 0.0 "VTBlend_Linear" 0.0 false))

(event `CloseDoc`
  ; Open/Close Document Effect
  (`PlayerController.SetViewTargetWithBlend` (`GameplayStatics.GetPlayerController` 0) (`self.Player`) 0.0 "VTBlend_Linear" 0.0 false)
  (`self.ChangeMappings` "/Game/Input/IMC_Default.IMC_Default" "/Game/Input/IMC_Limited.IMC_Limited")
  (set `self.canQuit` false)
  (`ActorComponent.Deactivate` (`self.Camera`)))

(event `CanQuitUpdate`
  ; Open/Close Document Effect
  (set `self.canQuit` true))

(fn `ChangeMappings`
  (params (MappingContextToAdd :type "InputMappingContext Object Reference") (MappingContexToRemove :type "InputMappingContext Object Reference"))
  (bind _asbp_third_person_player_controller (cast `/Game/Blueprints/Core/BP_ThirdPersonPlayerController` (`GameplayStatics.GetPlayerController` 0)))
  (`/Game/Blueprints/Core/BP_ThirdPersonPlayerController.UpdateInputMapping` _asbp_third_person_player_controller MappingContextToAdd MappingContexToRemove))

(fn `CloseInteract`
  (params (Component :type "/Game/Blueprints/Characters/Components/AC_CharacterComponent Object Reference"))
  (if (`self.canQuit`)
    (clear `/Game/Blueprints/Characters/Components/AC_CharacterComponent.LimitedInteractHasBeenPressed` Component)
    (`Widget.RemoveFromParent` (`self.WidgetTextRef`))
    (`self.CameraEffect` false)))

(fn `Interact`
  (params (Player :type "Character Object Reference"))
  (`parent.Interact` Player)
  (`ActorComponent.Activate` (`self.Camera`) false)
  (set `self.Player` Player)
  (`self.CameraEffect` true)
  (`self.ChangeMappings` "/Game/Input/IMC_Limited.IMC_Limited" "/Game/Input/IMC_Default.IMC_Default")
  (add `/Game/Blueprints/Characters/Components/AC_CharacterComponent.LimitedInteractHasBeenPressed` (`self.GetComponentByClass` Player "/Game/Blueprints/Characters/Components/AC_CharacterComponent.AC_CharacterComponent_C") (`|CreateDelegate` :!event `CloseInteract`)))

(fn `UserConstructionScript`
  (`parent.UserConstructionScript`))
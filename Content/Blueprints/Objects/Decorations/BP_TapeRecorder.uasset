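; BP_TapeRecorder is a main menu decoration that reacts when the Start Game button is hovered.
; On BeginPlay it waits for GM_MainMenu's MainMenuReady event before binding to the button's hover and unhover delegates.
; Hovering and unhovering handlers each play a one-shot start or stop recording animation on the skeletal mesh and swap its material to match.
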(event `BindEvenrs`
  (bind _wbp_startgame (`/Game/Blueprints/Widgets/WBP_MainMenu.WBP_StartGame` (`/Game/Blueprints/Core/Menu/GM_MainMenu.MainMenuRef` (stale `self.ReceiveBeginPlay` _asgm_main_menu))))
  (add `/Game/Blueprints/Widgets/WBP_ButtonBase.OnButtonHovered` _wbp_startgame (`|CreateDelegate` :!event `HoveringNewGame`))
  (add `/Game/Blueprints/Widgets/WBP_ButtonBase.OnButtonUnhovered` _wbp_startgame (`|CreateDelegate` :!event `StopHoveringNewGame`)))

(event `self.ReceiveBeginPlay`
  (bind _asgm_main_menu (cast `/Game/Blueprints/Core/Menu/GM_MainMenu` (`GameplayStatics.GetGameMode`)))
  (add `/Game/Blueprints/Core/Menu/GM_MainMenu.MainMenuReady` _asgm_main_menu (delegate `BindEvenrs`)))

(event `HoveringNewGame`
  (`SkeletalMeshComponent.PlayAnimation` (`self.SkeletalMesh`) "/Game/Assets/Anim/Tape/AM_StartRec.AM_StartRec" false)
  (`PrimitiveComponent.SetMaterial` (`self.SkeletalMesh`) 0 "/Game/VLCG_TapeRecorder/MaterialIstances/MI_TapeRecorder_A1.MI_TapeRecorder_A1"))

(event `StopHoveringNewGame`
  (bind _skeletalmesh (`self.SkeletalMesh`))
  (`SkeletalMeshComponent.PlayAnimation` _skeletalmesh "/Game/Assets/Anim/Tape/AS_RecStop.AS_RecStop" false)
  (`PrimitiveComponent.SetMaterial` _skeletalmesh 0 "/Game/VLCG_TapeRecorder/MaterialIstances/MI_TapeRecorder_A2.MI_TapeRecorder_A2"))

(fn `UserConstructionScript`)